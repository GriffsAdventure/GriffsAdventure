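; Enemy actor that turns to face a seen player character and fires projectiles at it, intended to patrol between random points.
; Pawn sensing drives the look-at rotation and impulse-launched BP_Projectile shots, throttled by a flag and delay.
; BeginPlay caches three marker positions and picks a random index.
; The PatrolTimeline logic that lerps toward that point and re-rolls it is never started in this graph.
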(event OnSeePawn(PawnSensing)
  (params (Pawn :type Pawn%20Object%20Reference))
  ;[1 1 1] LookAtAndShootPawn
  (bind _asthird_person_character (Utilities|Casting|CastToThirdPersonCharacter Pawn))
  (Utilities|FlowControl|Sequence
    (:then_0
      (Transformation|SetActorRotation (Math|Rotator|FindLookatRotation (Transformation|GetActorLocation) (Transformation|GetActorLocation _asthird_person_character))))
    (:then_1
      (if (Variables|Default|GetSpawnProjectile)
        (bind _returnvalue (Game|SpawnActorfromClass "/Game/Blueprints/BP_Projectile.BP_Projectile_C" (Transformation|GetWorldTransform (Variables|Default|GetProjectSpawnLocation)) "Undefined" 0 0))
        (Physics|AddImpulse (Variables|/Game/Blueprints/BP_Projectile.BP_Projectile_C|GetSphere _returnvalue) (* (Math|Vector|GetForwardVector (Variables|Default|GetCube)) (Variables|Default|GetShootAmount)) "None" true)
        (Variables|Default|SetSpawnProjectile false)
        (Utilities|FlowControl|Delay 1.5)
        (Variables|Default|SetSpawnProjectile true)))))

(event EventBeginPlay
  ;[1 1 1] SetPatrolPoints
  (Variables|Default|SetPatrolPoints (Utilities|Array|MakeArray (Transformation|GetWorldLocation (Variables|Default|GetMovePosition1)) (Transformation|GetWorldLocation (Variables|Default|GetMovePosition2)) (Transformation|GetWorldLocation (Variables|Default|GetMovePosition3))))
  (CallFunction|GetRandomLocation))

(fn ConstructionScript)

(fn GetRandomLocation
  (Variables|Default|SetCurrentPatrolPoint (Math|Random|RandomInteger (Utilities|Array|Length (Variables|Default|GetPatrolPoints)))))